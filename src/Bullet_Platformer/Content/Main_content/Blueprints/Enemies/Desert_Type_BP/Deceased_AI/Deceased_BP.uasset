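; Paper2D Blueprint for the Deceased, a desert-type enemy that animates by swapping flipbooks.
; Tick plays the moving flipbook until PawnSensing spots a pawn, which triggers the attack flipbook and a two-second CanAttack delay.
; Separate events offer a Moving/Idle state selector and a forward sphere-trace attack animation, neither called here nor dealing damage.
; BeginPlay copies Health to the health bar widget; the sphere overlap only casts to the player.
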(event OnSeePawn(PawnSensing)
  (params (Pawn :type Pawn%20Object%20Reference))
  (Variables|Default|SetisSeeingPlayer? true)
  (CallFunction|AttackPlayer))

(event OnComponentBeginOverlap(Sphere)
  (params (OverlappedComponent :type Primitive%20Component%20Object%20Reference) (OtherActor :type Actor%20Object%20Reference) (OtherComp :type Primitive%20Component%20Object%20Reference) (OtherBodyIndex :type Integer) (bFromSweep :type Boolean) (SweepResult :type Hit%20Result%20Structure%20%28by%20ref%29))
  (Utilities|Casting|CastToPlayer_Char_BP OtherActor))

(event Custom|Attack%20player%20Deceased
  (bind _returnvalue (Transformation|GetActorLocation))
  (bind _outhit (Collision|SphereTraceForObjects _returnvalue (+ _returnvalue (* (Math|Vector|GetForwardVector (Transformation|GetActorRotation)) 2.5e+02)) 0.0 (Utilities|Array|MakeArray "ObjectTypeQuery3") false 0 "ForDuration"))
  (if true
    (Utilities|Casting|CastToPaperCharacter (.HitActor (Collision|BreakHitResult _outhit)))
    (Sprite|SetFlipbook (Variables|Default|GetSprite) "/Game/Main_content/Assets/Textures/Enemies/Desert_Type_Enemies/Deceased/Deceased_attack_animation.Deceased_attack_animation")
    (Utilities|FlowControl|Delay 2.0)
    (Variables|Default|SetcanAttack? true)))

(event Custom|Dec_UpdateAnimation
  (bind _output_get (Variables|Default|SetisMoving? (> (Math|Vector|VectorLength (Transformation|GetVelocity)) 0.0)))
  (bind _output_flipbook (CallFunction|DecAnimStateMachine _output_get false false))
  (Sprite|SetFlipbook (Variables|Default|GetSprite) _output_flipbook))

(event Custom|AttackPlayer
  (if (Variables|Default|GetisSeeingPlayer?)
    (Variables|Default|SetcanAttack? false)
    (Sprite|SetFlipbook (Variables|Default|GetSprite) (Variables|Animation|GetattackFlipBook))
    (Utilities|FlowControl|Delay 2.0)
    (Variables|Default|SetcanAttack? true)
    (else
      (Variables|Default|SetisSeeingPlayer? false))))

(event EventBeginPlay
  (CallFunction|DecHealthBarUpdate))

(event Collision|EventActorBeginOverlap
  (params (OtherActor :type Actor%20Object%20Reference)))

(event EventTick
  (params (DeltaSeconds :type Float%20%28single-precision%29))
  (if (not (Variables|Default|GetisSeeingPlayer?))
    (Sprite|SetFlipbook (Variables|Default|GetSprite) (Variables|Animation|GetmovingFlipBook))))

(fn ConstructionScript)

(fn DecAnimStateMachine
  (params (is%20Moving? :type Boolean) (canAttack? :type Boolean) (isDead? :type Boolean))
  (if is%20Moving?
    (Variables|Default|SetAnimationState "NewEnumerator0")
    (else
      (Variables|Default|SetAnimationState "NewEnumerator1")))
  (return (Utilities|Select :Index (Variables|Default|GetAnimationState) :NewEnumerator0 (Variables|Animation|GetmovingFlipBook) :NewEnumerator1 (Variables|Animation|GetidleFlipBook) :NewEnumerator2 (Variables|Animation|GethurtFlipBook) :NewEnumerator3 (Variables|Animation|GetattackFlipBook) :NewEnumerator4 (Variables|Animation|GetdeathFlipBook))))

(fn DecHealthBarUpdate
  (bind _asdeceased_healthbar (Utilities|Casting|CastToDeceased_Healthbar (UserInterface|GetUserWidgetObject (Variables|Default|GetWidget))))
  (Utilities|IsValid _asdeceased_healthbar
    (:Is%20Valid
      (Variables|/Game/Main_content/Blueprints/Enemies/Desert_Type_BP/Deceased_AI/Deceased_Healthbar.Deceased_Healthbar_C|SetHealth _asdeceased_healthbar (Variables|Default|GetHealth))
      (return))))