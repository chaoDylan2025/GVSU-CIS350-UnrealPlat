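; Mummy enemy Blueprint that spots the player and has a partly wired melee attack and health bar.
; Pawn sensing sets a blackboard flag on its AI controller when it sees the PaperCharacter.
; MummyAttackPlayer runs a forward debug sphere trace for pawns, but does nothing after casting the hit actor.
; Tick only fetches the health bar widget; the percent update and camera-facing rotation are disconnected and never run.
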(event OnSeePawn(PawnSensing)
  (params (Pawn :type Pawn%20Object%20Reference))
  (Utilities|Casting|CastToPaperCharacter Pawn)
  (AI|Components|Blackboard|SetValueasBool (AI|GetBlackboard (AI|GetAIController self)) (Utilities|Name|MakeLiteralName "hasSeenPlayer4") true))

(event Custom|Mummy%20Attack%20Player
  (bind _returnvalue (Transformation|GetActorLocation))
  (bind _outhit (Collision|SphereTraceForObjects _returnvalue (+ _returnvalue (* (Math|Vector|GetForwardVector (Transformation|GetActorRotation)) 2.5e+02)) 0.0 (Utilities|Array|MakeArray "ObjectTypeQuery3") false 0 "ForDuration"))
  (if true
    (Utilities|Casting|CastToPaperCharacter (.HitActor (Collision|BreakHitResult _outhit)))))

(event EventBeginPlay)

(event Collision|EventActorBeginOverlap
  (params (OtherActor :type Actor%20Object%20Reference)))

(event EventTick
  (params (DeltaSeconds :type Float%20%28single-precision%29))
  (bind _asmummy_healthbar (Utilities|Casting|CastToMummy_Healthbar (UserInterface|GetWidget (Variables|Default|GetWidget)))))

(fn ConstructionScript)