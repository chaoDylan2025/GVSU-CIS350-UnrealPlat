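; Player character for a side-view flipbook blue wizard with walking, double jump, stamina-costed dash and melee attack.
; Enhanced Input drives movement and jumping, flipping the sprite for facing and polling Z velocity to detect landing.
; Left-click attacks damage overlapping Deceased_BP actors every Tick until the animation finishes; dash steps through swept moves in a delayed-loop macro.
; Retriggerable-delay loops regenerate stamina and HP after key release, with F applying self-damage.
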(event OnFinishedPlaying(Sprite)
  (Sprite|SetFlipbook (Variables|Default|GetSprite) "/Game/Main_content/Assets/BlueWizardIdle.BlueWizardIdle")
  (Components|Timeline|SetLooping (Variables|Default|GetSprite) true)
  (if (not (Audio|Components|Audio|IsPlaying (Variables|Default|GetSprite)))
    (Audio|Components|Audio|Play (Variables|Default|GetSprite))
    (Variables|Default|SetisAttacking false)))

(event Custom|Dash
  (bind _returnvalue (Transformation|GetActorRotation))
  (if (>= (Variables|Default|GetStamina) 2e+01)
    (if (Variables|Default|Getrotated)
      (Utilities|ForLoopwithDelay 0 20 0.0005
        (:Body
          (Transformation|SetActorLocationAndRotation (+ (Transformation|GetWorldLocation (Variables|Default|GetSprite)) "-8.000000,0.000000,0.000000") _returnvalue true))
        (:Completed
          (Variables|Default|SetStamina (- (Variables|Default|GetStamina) 2e+01) :!label _label)))
      (else
        (Utilities|ForLoopwithDelay 0 20 0.0005
          (:Body
            (Transformation|SetActorLocationAndRotation (+ (Transformation|GetWorldLocation (Variables|Default|GetSprite)) "8.000000,0.000000,0.000000") _returnvalue true))
          (:Completed
            (goto _label)))))))

(event Custom|TakeDamage
  (params (Damage_Taken :type Float%20%28double-precision%29))
  (Variables|Default|SetHP (- (Variables|Default|GetHP) Damage_Taken)))

(event Custom|IncreaseStamina
  (Variables|Default|SetStamina (+ (Variables|Default|GetStamina) 2.0))
  (if (>= (Variables|Default|GetStamina) 1e+02)
    (Variables|Default|SetcanStaminaIncrease? false)
    (else
      (Variables|Default|SetcanStaminaIncrease? true))))

(event Custom|IncreaseHP
  (Variables|Default|SetHP (+ (Variables|Default|GetHP) 1e+01))
  (if (>= (Variables|Default|GetHP) 1e+02)
    (Variables|Default|SetcanHPIncrease false)
    (else
      (Variables|Default|SetcanHPIncrease true))))

(event Input|EnhancedActionEvents|EnhancedInputActionBase_char_movement
  (params (ActionValue :type Float%20%28double-precision%29) (ElapsedSeconds :type Float%20%28double-precision%29) (TriggeredSeconds :type Float%20%28double-precision%29) (InputAction :type Input%20Action%20Object%20Reference :default "/Game/Main_content/Blueprints/Base_char_movement.Base_char_movement"))
  (:Triggered
    (if (Variables|Default|Getis_Jump)
      _
      (else
        _))
    (Pawn|Input|AddMovementInput (Transformation|GetActorForwardVector) ActionValue false)
    (Sprite|SetFlipbook (Variables|Default|GetSprite) "/Game/Main_content/Assets/BlueCharWalk.BlueCharWalk")
    (if (> ActionValue 0.0)
      (Transformation|SetWorldRotation (Variables|Default|GetSprite) "0, 0, 0" false false)
      (Variables|Default|Setrotated false)
      (else
        (Transformation|SetWorldRotation (Variables|Default|GetSprite) "0.000000,-180.000000,0.000000" false false)
        (Variables|Default|Setrotated true))))
  (:Completed
    (if (not (Variables|Default|Getis_Jump))
      (Sprite|SetFlipbook (Variables|Default|GetSprite) "/Game/Main_content/Assets/BlueWizardIdle.BlueWizardIdle"))))

(event Input|EnhancedActionEvents|EnhancedInputActionBase_char_Jump
  (params (ActionValue :type Boolean) (ElapsedSeconds :type Float%20%28double-precision%29) (TriggeredSeconds :type Float%20%28double-precision%29) (InputAction :type Input%20Action%20Object%20Reference :default "/Game/Main_content/Blueprints/Base_char_Jump.Base_char_Jump"))
  (bind _sprite (Variables|Default|GetSprite))
  (if (Variables|Default|Getis_Jump)
    (if (not (Variables|Default|GetdoubleJump))
      (Variables|Default|SetdoubleJump true)
      (Character|StopJumping)
      (Character|Jump :!label _label)
      (Components|Timeline|SetLooping _sprite false)
      (Sprite|SetFlipbook _sprite "/Game/Main_content/Assets/BlueChatJump.BlueChatJump")
      (Utilities|FlowControl|Delay 0.1)
      (if (== (.Z (Math|Vector|BreakVector (Transformation|GetVelocity))) 0.0) :!label _label_2
        (Components|Timeline|SetLooping _sprite true)
        (Audio|Components|Audio|Play _sprite)
        (Sprite|SetFlipbook _sprite "/Game/Main_content/Assets/BlueWizardIdle.BlueWizardIdle")
        (Variables|Default|Setis_Jump false)
        (Variables|Default|SetdoubleJump false)
        (else
          (Utilities|FlowControl|Delay 0.1)
          (goto _label_2))))
    (else
      (Variables|Default|Setis_Jump true)
      (goto _label))))

(event EventBeginPlay
  (bind _asplayer_controller_bp (Utilities|Casting|CastToPlayer_controller_BP (Pawn|GetController)))
  (Input|AddMappingContext (PlayerController|LocalPlayerSubsystems|GetEnhancedInputLocalPlayerSubsystem _asplayer_controller_bp) "/Game/Main_content/Blueprints/Input_map_default.Input_map_default" 0 "(bIgnoreAllPressedKeysUntilRelease=True,bForceImmediately=False,bNotifyUserSettings=False)"))

(event EventTick
  (params (DeltaSeconds :type Float%20%28single-precision%29))
  (if (Variables|Default|GetisAttacking)
    (CallFunction|HitCheck)))

(event Input|KeyboardEvents|LeftShift
  (params (Key :type Key%20Structure :default "None"))
  (:Pressed
    (CallFunction|Dash)
    (Variables|Default|SetStamina_in_use true)
    (Development|PrintText (Utilities|Text|ToText(Float) (Variables|Default|GetStamina) "HalfToEven")))
  (:Released
    (Utilities|FlowControl|RetriggerableDelay 0.2 :!label _label)
    (CallFunction|IncreaseStamina)
    (if (Variables|Default|GetcanStaminaIncrease?)
      (goto _label))))

(event Input|KeyboardEvents|F
  (params (Key :type Key%20Structure :default "None"))
  (:Pressed
    (CallFunction|TakeDamage 2e+01))
  (:Released
    (Utilities|FlowControl|RetriggerableDelay 4.0 :!label _label)
    (CallFunction|IncreaseHP)
    (if (Variables|Default|GetcanHPIncrease)
      (goto _label))))

(event Input|MouseEvents|LeftMouseButton
  (params (Key :type Key%20Structure :default "None"))
  (:Pressed
    (Sprite|SetFlipbook (Variables|Default|GetSprite) "/Game/Main_content/Assets/BlueWizardAttack.BlueWizardAttack")
    (Components|Timeline|SetLooping (Variables|Default|GetSprite) false)
    (Variables|Default|SetisAttacking true)))

(fn ConstructionScript)

(fn HitCheck
  (for _array_element (Collision|GetOverlappingActors (Variables|Default|GetAttack_box) "/Game/Main_content/Blueprints/Enemies/Desert_Type_BP/Deceased_AI/Deceased_BP.Deceased_BP_C" :!class /Script/Engine.PrimitiveComponent)
    (if (!= _array_element self)
      (Game|Damage|ApplyDamage _array_element (Variables|Default|GetBase%20Damage) 0 0))))